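; BP_SOCRTSPawn is the SOC RTS player pawn, currently handling only mouse cursor and input setup.
; On BeginPlay it shows the cursor, sets Game and UI input locked to the viewport, ignores look input and captures the mouse permanently.
; Each Tick it prints the mouse position as a debug string, with no camera movement or selection logic in this graph.
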(event `self.ReceiveBeginPlay`
  (`parent.ReceiveBeginPlay`)
  (bind _asplayer_controller (cast `PlayerController` (`self.GetController`)))
  (set `PlayerController.bShowMouseCursor` true _asplayer_controller)
  (`WidgetBlueprintLibrary.SetInputMode_GameAndUIEx` _asplayer_controller null "LockAlways" false)
  (`Controller.SetIgnoreLookInput` _asplayer_controller true)
  (`GameplayStatics.SetViewportMouseCaptureMode` "CapturePermanently"))

(event `self.ReceiveTick`
  (params (DeltaSeconds :type "Float (single-precision)"))
  (bind _asplayer_controller (cast `PlayerController` (`self.GetController`)))
  (bind (_locationx _locationy) (`PlayerController.GetMousePosition` _asplayer_controller))
  (`KismetSystemLibrary.PrintString` (`KismetStringLibrary.Conv_Vector2dToString` (`KismetMathLibrary.MakeVector2D` _locationx _locationy))))

(fn `UserConstructionScript`)