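; Player rematch objective that drives the rematch ready-check UI on the local HUD.
; On Begin for an assigned local player, it creates WBP_RematchCheck, stores it on SOCHUD, notifies it and subscribes to game state match-state changes.
; Status changes ensure the widget exists, refresh ready status and pass whether all assignees completed the tagged objectives.
; When the match returns to Waiting to Start, the widget is removed from screen.
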(event `SetupOnRematchEvent`
  (bind _assocgame_state (cast `SOCGameState` (`GameplayStatics.GetGameState`)))
  (add `SOCGameState.GameStateMatchStateSetEvent` _assocgame_state (delegate `GameStateMatchStateSetEvent_Event`)))

(event `GameStateMatchStateSetEvent_Event`
  (params (MatchState :type Name))
  (switch `name` MatchState
    (:`WaitingToStart`
      (bind _assochud (cast `SOCHUD` (`PlayerController.GetHUD` (`GameplayStatics.GetPlayerController` 0))))
      (bind _returnvalue (`SOCHUD.GetRematchCheckWidget` _assochud))
      (`/Engine/EditorBlueprintResources/StandardMacros.IsValid` _returnvalue
        (:`Is Valid`
          (`Widget.RemoveFromParent` _returnvalue))))))

(event `self.K2_Begin`
  (params (Assignee :type "Actor Object Reference"))
  (`|ExecutionSequence`
    (:`then_0`
      (bind _asplayer_state (cast `PlayerState` Assignee))
      (bind _returnvalue (`PlayerState.GetPlayerController` _asplayer_state))
      (`/Engine/EditorBlueprintResources/StandardMacros.IsValid` _returnvalue
        (:`Is Valid`
          (if (`Controller.IsLocalPlayerController` _returnvalue)
            (if (`self.IsAssigned` _asplayer_state)
              (`self.SetupObjectiveWidget`))))))
    (:`then_1`
      (bind _assochud (cast `SOCHUD` (`PlayerController.GetHUD` (`GameplayStatics.GetPlayerController` 0))))
      (bind _rematchcheckwidget (`SOCHUD.RematchCheckWidget` _assochud)
        (:`then`
          (bind _aswbp_rematch_check (cast `/Game/SOC/HUD/Widgets/RematchCheck/WBP_RematchCheck` _rematchcheckwidget))
          (`/Game/SOC/HUD/Widgets/RematchCheck/WBP_RematchCheck.OnBeginObjective` _aswbp_rematch_check))
        (:`else`)))
    (:`then_2`
      (`self.SetupOnRematchEvent`))))

(event `self.K2_OnObjectiveStatusesChanged`
  (`|ExecutionSequence`
    (:`then_0`
      (`self.SetupObjectiveWidget`)
      (bind _assochud (cast `SOCHUD` (`PlayerController.GetHUD` (`GameplayStatics.GetPlayerController` 0))))
      (bind _rematchcheckwidget (`SOCHUD.RematchCheckWidget` _assochud)
        (:`then`
          (bind _aswbp_rematch_check (cast `/Game/SOC/HUD/Widgets/RematchCheck/WBP_RematchCheck` _rematchcheckwidget))
          (`/Game/SOC/HUD/Widgets/RematchCheck/WBP_RematchCheck.UpdateReadyCheckStatus` _aswbp_rematch_check))
        (:`else`)))
    (:`then_1`
      (bind _assochud_2 (cast `SOCHUD` (`PlayerController.GetHUD` (`GameplayStatics.GetPlayerController` 0))))
      (bind _rematchcheckwidget_2 (`SOCHUD.RematchCheckWidget` _assochud_2)
        (:`then`
          (bind _aswbp_rematch_check_2 (cast `/Game/SOC/HUD/Widgets/RematchCheck/WBP_RematchCheck` _rematchcheckwidget_2))
          (`/Game/SOC/HUD/Widgets/RematchCheck/WBP_RematchCheck.OnAllPlayersReady` _aswbp_rematch_check_2 (`.ReturnValue` (`ObjectiveSystemBlueprintLibrary.HaveAllAssigneesCompletedObjectivesByTags` (`self.ObjectiveTags`)))))
        (:`else`)))))

(fn `SetupObjectiveWidget`
  ;[1 1 1] TODO: Move this code and widget class storage to the HUD class
  (bind _assochud (cast `SOCHUD` (`PlayerController.GetHUD` (`GameplayStatics.GetPlayerController` 0))))
  (`SOCHUD.RematchCheckWidget` _assochud
    (:`then`)
    (:`else`
      (bind _returnvalue (`|CreateWidget` "/Game/SOC/HUD/Widgets/RematchCheck/WBP_RematchCheck.WBP_RematchCheck_C" (`GameplayStatics.GetPlayerController` 0)))
      (`SOCHUD.SetRematchCheckWidget` _assochud _returnvalue)
      (`UserWidget.AddToViewport` _returnvalue 0))))

(fn `UserConstructionScript`)