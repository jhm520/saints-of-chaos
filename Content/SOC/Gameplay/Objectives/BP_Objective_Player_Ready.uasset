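; Player ready-check objective that drives the ready-check widget on the local player's HUD.
; When the objective begins for an assigned local player, or statuses change, it creates WBP_ReadyCheck if missing.
; Status changes also refresh the widget and report whether all assignees completed objectives matching its tags.
; It binds to game state match changes, waiting for game state if needed, and removes the widget once In Progress.
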(event `self.ReceiveBeginPlay`
  (bind _returnvalue (`GameplayStatics.GetGameState`))
  (`/Engine/EditorBlueprintResources/StandardMacros.IsValid` _returnvalue
    (:`Is Valid`
      (`self.OnGameStateHasBegunPlayDelegate_Event` _returnvalue))
    (:`Is Not Valid`
      (bind _assocgame_instance (cast `SOCGameInstance` (`GameplayStatics.GetGameInstance`)))
      (add `SOCGameInstance.OnGameStateHasBegunPlayDelegate` _assocgame_instance (delegate `OnGameStateHasBegunPlayDelegate_Event`)))))

(event `OnGameStateHasBegunPlayDelegate_Event`
  (params (GameState :type "GameStateBase Object Reference"))
  (bind _assocgame_state (cast `SOCGameState` GameState))
  (add `SOCGameState.GameStateMatchStateSetEvent` _assocgame_state (delegate `GameStateMatchStateSetEvent_Event`)))

(event `GameStateMatchStateSetEvent_Event`
  (params (MatchState :type Name))
  (switch `name` MatchState
    (:`InProgress`
      (bind _assochud (cast `SOCHUD` (`PlayerController.GetHUD` (`GameplayStatics.GetPlayerController` 0))))
      (bind _readycheckwidget (`SOCHUD.ReadyCheckWidget` _assochud)
        (:`then`
          (`Widget.RemoveFromParent` _readycheckwidget))
        (:`else`)))))

(event `self.K2_Begin`
  (params (Assignee :type "Actor Object Reference"))
  (`|ExecutionSequence`
    (:`then_0`
      (bind _asplayer_state (cast `PlayerState` Assignee))
      (bind _returnvalue (`PlayerState.GetPlayerController` _asplayer_state))
      (`/Engine/EditorBlueprintResources/StandardMacros.IsValid` _returnvalue
        (:`Is Valid`
          (if (`Controller.IsLocalPlayerController` _returnvalue)
            (if (`self.IsAssigned` Assignee)
              (`self.SetupObjectiveWidget`))))))))

(event `self.K2_OnObjectiveStatusesChanged`
  (`|ExecutionSequence`
    (:`then_0`
      (`self.SetupObjectiveWidget`)
      (bind _assochud (cast `SOCHUD` (`PlayerController.GetHUD` (`GameplayStatics.GetPlayerController` 0))))
      (bind _readycheckwidget (`SOCHUD.ReadyCheckWidget` _assochud)
        (:`then`
          (bind _aswbp_ready_check (cast `/Game/SOC/HUD/Widgets/ReadyCheck/WBP_ReadyCheck` _readycheckwidget))
          (`/Game/SOC/HUD/Widgets/ReadyCheck/WBP_ReadyCheck.UpdateReadyCheckStatus` _aswbp_ready_check))
        (:`else`)))
    (:`then_1`
      (bind _assochud_2 (cast `SOCHUD` (`PlayerController.GetHUD` (`GameplayStatics.GetPlayerController` 0))))
      (bind _readycheckwidget_2 (`SOCHUD.ReadyCheckWidget` _assochud_2)
        (:`then`
          (bind _aswbp_ready_check_2 (cast `/Game/SOC/HUD/Widgets/ReadyCheck/WBP_ReadyCheck` _readycheckwidget_2))
          (`/Game/SOC/HUD/Widgets/ReadyCheck/WBP_ReadyCheck.OnAllPlayersReady` _aswbp_ready_check_2 (`.ReturnValue` (`ObjectiveSystemBlueprintLibrary.HaveAllAssigneesCompletedObjectivesByTags` (`self.ObjectiveTags`)))))
        (:`else`)))))

(event `SetupObjectiveWidget`
  (bind _assochud (cast `SOCHUD` (`PlayerController.GetHUD` (`GameplayStatics.GetPlayerController` 0))))
  (`SOCHUD.ReadyCheckWidget` _assochud
    (:`then`)
    (:`else`
      (bind _returnvalue (`|CreateWidget` "/Game/SOC/HUD/Widgets/ReadyCheck/WBP_ReadyCheck.WBP_ReadyCheck_C" (`GameplayStatics.GetPlayerController` 0)))
      (`SOCHUD.SetReadyCheckWidget` _assochud _returnvalue)
      (`UserWidget.AddToViewport` _returnvalue 0))))

(fn `UserConstructionScript`)