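; Gameplay ability for a mob's sword melee attack, dealing randomized damage to a single target.
; On commit it gets instant target data from a single-actor target actor and plays the auto-attack montage.
; After a fixed delay timed from montage start, it applies the damage effect with a random negative SetByCaller magnitude.
; The ability ends when the montage completes, is interrupted or cancelled, or targeting is cancelled.
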(event `self.K2_ActivateAbility`
  (`KismetSystemLibrary.PrintString` "Melee Attack")
  (bind _returnvalue (`self.K2_CommitAbility`))
  (if _returnvalue
    (bind (_asynctaskproxy _data) (`AbilityTask_WaitTargetData.WaitTargetData` "None" "Instant" "/Script/GASUtility.GameplayAbilityTargetActor_SingleActor" (struct) (struct) null)
      (:`ValidData`
        (`AbilityTask_PlayMontageAndWait.CreatePlayMontageAndWaitProxy` "None" "/Game/SOC/Characters/Mob/Animations/Sword/AM_Mob_Sword_AutoAttack.AM_Mob_Sword_AutoAttack" 1.0 "None" false
          (:`then`
            (`GameplayTask_WaitDelay.TaskWaitDelay` null 0.85
              (:`OnFinish`
                (bind _returnvalue_2 (`AbilitySystemBlueprintLibrary.AssignTagSetByCallerMagnitude` (`self.MakeOutgoingGameplayEffectSpec` (`self.MeleeAttackGameplayEffect`)) (struct :`TagName` "Mob.Ability.MeleeAttack.Damage") (`KismetMathLibrary.RandomFloatInRange` -60.0 -23.0)))
                (`self.K2_ApplyGameplayEffectSpecToTarget` _returnvalue_2 _data))))
          (:`OnCompleted`
            (`self.K2_EndAbility`))
          (:`OnInterrupted`
            (`self.K2_EndAbility` :!label _label))
          (:`OnCancelled`
            (goto _label))))
      (:`Cancelled`
        (`self.K2_EndAbility`)))))