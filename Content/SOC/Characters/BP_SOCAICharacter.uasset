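; BP_SOCAICharacter is an AI character that shows a selection indicator when a player selects it.
; Its SelectableComponent's selected and deselected delegates unhide and hide a ChildActor.
; Both handlers cast the selector to Pawn and act only when it is locally controlled, so the indicator appears just for the player who made the selection.
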(event `self.ReceiveBeginPlay`)

(event `self.ReceiveTick`
  (params (DeltaSeconds :type "Float (single-precision)")))

(event `self.SelectableComponent.OnSelectedDelegate`
  (params (Selector :type "Actor Object Reference"))
  (bind _aspawn (cast `Pawn` Selector))
  (if (`self.IsLocallyControlled` _aspawn)
    (`SceneComponent.SetHiddenInGame` (`self.ChildActor`) false false)))

(event `self.SelectableComponent.OnDeselectedDelegate`
  (params (Selector :type "Actor Object Reference"))
  (bind _aspawn (cast `Pawn` Selector))
  (if (`self.IsLocallyControlled` _aspawn)
    (`SceneComponent.SetHiddenInGame` (`self.ChildActor`) true false)))

(fn `UserConstructionScript`)