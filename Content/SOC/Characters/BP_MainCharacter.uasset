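; BP_MainCharacter is a playable character with camera-relative movement and a controller-driven orbit camera.
; Camera axis inputs add controller pitch and yaw, and Tick copies the control rotation to SpringArmPivot's world rotation.
; Move axes add movement along the camera's forward and right vectors with Z zeroed, without renormalizing.
; Leftover public and local IP lookup nodes are unconnected and never run.
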(event `self.ReceiveTick`
  (params (DeltaSeconds :type "Float (single-precision)"))
  (`parent.ReceiveTick` DeltaSeconds)
  (`self.UpdateCameraPivot`))

(event `InputAxis|CameraUpAction`
  (params (AxisValue :type "Float (single-precision)"))
  (`self.AddControllerPitchInput` AxisValue))

(event `InputAxis|CameraRightAction`
  (params (AxisValue :type "Float (single-precision)"))
  (`self.AddControllerYawInput` AxisValue))

(event `InputAxis|MoveForwardAction`
  (params (AxisValue :type "Float (single-precision)"))
  (`self.AddMovementInput` (* (`SceneComponent.GetForwardVector` (`self.Camera`)) (1.0 1.0 0.0)) AxisValue))

(event `InputAxis|MoveRightAction`
  (params (AxisValue :type "Float (single-precision)"))
  (`self.AddMovementInput` (* (`SceneComponent.GetRightVector` (`self.Camera`)) (1.0 1.0 0.0)) AxisValue))

(fn `UpdateCameraPivot`
  (`SceneComponent.K2_SetWorldRotation` (`self.SpringArmPivot`) (`self.GetControlRotation`) false false))

(fn `UserConstructionScript`)